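; HealthPickup is a pickup actor that restores health to any CharacterBase that overlaps it.
; On overlap it adds HealthPickupValue to the character's Health, then destroys itself.
; The maximum is read from the Health class default of the character's own class, so healing is capped at that value.
; Characters whose Health already equals that default leave the pickup in place.
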(event `self.ReceiveActorBeginOverlap`
  (params (OtherActor :type "Actor Object Reference"))
  (bind _ascharacter_base (cast `/Game/Blueprints/Characters/CharacterBase` OtherActor))
  (bind _health (defaults `/Game/Blueprints/Pickups/HealthPickup` (`GameplayStatics.GetObjectClass` _ascharacter_base)))
  (if (not (== _health (`/Game/Blueprints/Characters/CharacterBase.Health` _ascharacter_base)))
    (set `/Game/Blueprints/Characters/CharacterBase.Health` (`KismetMathLibrary.FMin` (+ (`/Game/Blueprints/Characters/CharacterBase.Health` _ascharacter_base) (`self.HealthPickupValue`)) _health) _ascharacter_base)
    (`self.K2_DestroyActor`)))

(fn `UserConstructionScript`)