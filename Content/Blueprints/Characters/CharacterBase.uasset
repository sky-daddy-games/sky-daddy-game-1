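; Base character with health, sword melee, magic projectile attacks and a customizable hair color.
; It spawns a socketed sword, links a health bar widget to itself, and drives attacks through montages with section-based combo chaining.
; Damage triggers flinches that block attacks, except during listed attack sections.
; Death destroys sword and character, ending the game if player-controlled; survivors play a victory montage on the game mode's end-game dispatch.
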(event `CreateSword`
  (bind _returnvalue (`|SpawnActorFromClass` "/Game/Blueprints/Weapons/BaseSword.BaseSword_C" (`self.GetTransform`) "Undefined" "OverrideRootScale" null null))
  (`self.K2_AttachToComponent` _returnvalue (`self.Mesh`) "Sword" "SnapToTarget" "SnapToTarget" "SnapToTarget" false)
  (set `self.Weapon` _returnvalue))

(event `self.ReceiveBeginPlay`
  (`self.CreateSword`)
  (`self.SetupHealth`)
  (bind _asprimary_game_mode (cast `/Game/Blueprints/GameModes/PrimaryGameMode` (`GameplayStatics.GetGameMode`)))
  (add `/Game/Blueprints/GameModes/PrimaryGameMode.EndGameDispatch` _asprimary_game_mode (delegate `EndGameDance`)))

(event `EndGameDance`
  (if (> (`self.Health`) 0.0)
    (`CharacterMovementComponent.DisableMovement` (`self.CharacterMovement`))
    (`self.PlayAnimMontage` "/Game/Assets/Knight/Anim/Montage_Victory.Montage_Victory")))

(event `TryMelee`
  (bind _returnvalue (`SkeletalMeshComponent.GetAnimInstance` (`self.Mesh`)))
  (bind _returnvalue_2 (`AnimInstance.Montage_GetCurrentSection` _returnvalue "/Game/Assets/Knight/Anim/Montage_Player_Attack.Montage_Player_Attack"))
  (if (`self.IsFlinching`)
    _
    (elif (`AnimInstance.Montage_IsActive` _returnvalue "/Game/Assets/Knight/Anim/Montage_Player_Attack.Montage_Player_Attack")
      (switch `name` _returnvalue_2
        (:`Attack1`
          (`AnimInstance.Montage_SetNextSection` _returnvalue _returnvalue_2 "Attack2" "/Game/Assets/Knight/Anim/Montage_Player_Attack.Montage_Player_Attack")))
      (else
        (`self.PlayAnimMontage` "/Game/Assets/Knight/Anim/Montage_Player_Attack.Montage_Player_Attack" 1.0 "Attack1")))))

(event `self.ReceiveAnyDamage`
  (params (Damage :type "Float (single-precision)") (DamageType :type "DamageType Object Reference") (InstigatedBy :type "Controller Object Reference") (DamageCauser :type "Actor Object Reference"))
  (bind _returnvalue (`SkeletalMeshComponent.GetAnimInstance` (`self.Mesh`)))
  (bind _output_get (set `self.Health` (- (`self.Health`) Damage)))
  (if (<= _output_get 0.0)
    (`/Engine/EditorBlueprintResources/StandardMacros.DoOnce` false
      (:`Completed`
        (set `self.IsFlinching` true)
        (`CharacterMovementComponent.DisableMovement` (`self.CharacterMovement`))
        (bind _returnvalue_2 (`self.PlayAnimMontage` "/Game/Assets/Knight/Anim/Montage_Player_Death.Montage_Player_Death"))
        (if (`Controller.IsPlayerController` (`self.GetController`))
          (`/Game/Blueprints/GameModes/PrimaryGameMode.EndGame` (cast `/Game/Blueprints/GameModes/PrimaryGameMode` (`GameplayStatics.GetGameMode`) :!pure true)))
        (`KismetSystemLibrary.Delay` _returnvalue_2)
        (`self.K2_DestroyActor` (`self.Weapon`))
        (`self.K2_DestroyActor`)))
    (else
      (set `self.IsFlinching` true)
      (if (`AnimInstance.Montage_IsActive` _returnvalue "/Game/Assets/Knight/Anim/Montage_Player_Attack.Montage_Player_Attack")
        (if (`KismetArrayLibrary.Array_Contains` (`self.AttackMoves`) (`AnimInstance.Montage_GetCurrentSection` _returnvalue "/Game/Assets/Knight/Anim/Montage_Player_Attack.Montage_Player_Attack"))
          (set `self.IsFlinching` false)
          (else
            (bind _returnvalue_3 (`self.PlayAnimMontage` "/Game/Assets/Knight/Anim/Montage_Player_Flinch.Montage_Player_Flinch" 1.0 "FlinchBig"))
            (`KismetSystemLibrary.Delay` _returnvalue_3)
            (set `self.IsFlinching` false :!label _label)))
        (else
          (bind _returnvalue_4 (`self.PlayAnimMontage` "/Game/Assets/Knight/Anim/Montage_Player_Flinch.Montage_Player_Flinch" 1.0 "FlinchSmall"))
          (`KismetSystemLibrary.Delay` _returnvalue_4)
          (goto _label))))))

(event `TryMagic`
  (if (not (`self.IsFlinching`))
    (`self.PlayAnimMontage` "/Game/Assets/Knight/Anim/Montage_Player_Shoot.Montage_Player_Shoot")))

(event `LaunchMagicProjectile`
  (`|SpawnActorFromClass` "/Game/Blueprints/Weapons/BaseProjectile.BaseProjectile_C" (`SceneComponent.K2_GetComponentToWorld` (`self.Arrow1`)) "Undefined" "OverrideRootScale" null self))

(event `UsePrimaryAttack`
  (`self.TryMelee`))

(event `SetupHealth`
  (bind _ashealth_bar (cast `/Game/Blueprints/Menus/HealthBar` (`WidgetComponent.GetUserWidgetObject` (`self.HealthBar`))))
  (`/Game/Blueprints/Menus/HealthBar.SetOwningCharacter` _ashealth_bar self))

(fn `UserConstructionScript`
  (bind _returnvalue (`PrimitiveComponent.CreateDynamicMaterialInstance` (`self.Mesh`) 0 null "None"))
  (`MaterialInstanceDynamic.SetVectorParameterValue` _returnvalue "HairColor" (`self.HairColor`))
  (`self.SetupHealth`))